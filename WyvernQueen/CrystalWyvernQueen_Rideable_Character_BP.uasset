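; Rideable Crystal Wyvern Queen character that adds key-triggered attacks and a water-activated aquatic buff.
; Entering a water volume adds the Spino aqua buff or holds it active; leaving has the server multicast a restart of its timed expiry.
; Water entry also line-traces for the surface to spawn scaled splash effects and sound.
; GetCrystalMeshes shows the skull mesh and returns the crystal, skull and other static meshes.
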(event Custom|Multi_UpdateBuffTime
  (params (bIsActive :type Boolean))
  (bind _returnvalue (Class|PrimalCharacter|GetBuff (Variables|Default|GetAquaticBuffClass)))
  (bind _asbuff_spinoaqua_c (Utilities|Casting|CastToBuff_SpinoAqua _returnvalue))
  (if bIsActive
    (Variables|/Script/ShooterGame.PrimalBuff|SetbUseTickingDeactivation _asbuff_spinoaqua_c false)
    (Variables|/Script/ShooterGame.PrimalBuff|SetDeactivateAfterTime _asbuff_spinoaqua_c 0.0)
    (else
      (Variables|/Script/ShooterGame.PrimalBuff|SetDeactivateAfterTime _asbuff_spinoaqua_c (Variables|/Game/PrimalEarth/CoreBlueprints/Buffs/Buff_SpinoAqua.Buff_SpinoAqua_C|GetAbilityCooldownTime _asbuff_spinoaqua_c))))
  (Class|PrimalBuff|ResetBuffStart _asbuff_spinoaqua_c))

(event EventActorBeginOverlap
  (params (OtherActor :type Actor%20Object%20Reference))
  (bind _asphysicsvolume (Utilities|Casting|CastToPhysicsVolume OtherActor))
  (if (Variables|/Script/Engine.PhysicsVolume|GetbWaterVolume _asphysicsvolume)
    (Utilities|FlowControl|Sequence
      (:then_0
        (bind _returnvalue (Class|PrimalCharacter|HasBuff (Variables|Default|GetAquaticBuffClass) false))
        (if (not _returnvalue)
          (Class|PrimalBuff|StaticAddBuff (Variables|Default|GetAquaticBuffClass) self 0 0 true)
          (else
            (CallFunction|MultiUpdateBuffTime true))))
      (:then_1
        (CallFunction|SpawnWaterOverlapVFX _asphysicsvolume)))))

(event EventActorEndOverlap
  (params (OtherActor :type Actor%20Object%20Reference))
  (if (Networking|IsServer)
    (bind _returnvalue (Class|PrimalCharacter|HasBuff (Variables|Default|GetAquaticBuffClass) false))
    (if _returnvalue
      (bind _asphysicsvolume (Utilities|Casting|CastToPhysicsVolume OtherActor))
      (if (Variables|/Script/Engine.PhysicsVolume|GetbWaterVolume _asphysicsvolume)
        (CallFunction|MultiUpdateBuffTime false)))))

(event Input|KeyboardEvents|X
  (:Pressed
    (Class|PrimalDinoCharacter|DoAttack 5 true false)))

(event Input|MouseEvents|MiddleMouseButton
  (:Pressed
    (Class|PrimalDinoCharacter|DoAttack 6 true false)))

(event Input|KeyboardEvents|G
  (:Pressed
    (Class|PrimalDinoCharacter|DoAttack 7 true false)))

(fn ConstructionScript
  (|CallParentFunction))

(fn SpawnWaterOverlapVFX
  (params (WaterActor :type Actor%20Object%20Reference))
  (bind _returnvalue (Transformation|GetActorLocation))
  (Class|KismetSystemLibrary|CanRunCosmeticEvents
    (:Yes
      (bind (_outhit _returnvalue_2) (Collision|LineTraceForObjects (+ _returnvalue "0, 0,265.000000") (- _returnvalue "0, 0,265.000000") (Utilities|Array|MakeArray "ObjectTypeQuery14") false 0 "None"))
      (if _returnvalue_2
        (if (== (.HitActor (Collision|BreakHitResult _outhit)) WaterActor)
          (bind _returnvalue_3 (Effects|SpawnEmitteratLocation "/Game/PrimalEarth/Effects/Particles/Water/FishingSplashLarge.FishingSplashLarge" (.ImpactPoint (Collision|BreakHitResult _outhit)) "0, 0,0.000000"))
          (Transformation|SetWorldScale3D _returnvalue_3 (Math|Vector|MakeVector 5.0 5.0 2.5))
          (Variables|/Script/Engine.ParticleSystemComponent|SetCustomTimeDilation _returnvalue_3 1.5)
          (bind _returnvalue_4 (Effects|SpawnEmitteratLocation "/Game/GunImpacts/Particles/P_ImpactWater_Large.P_ImpactWater_Large" (.ImpactPoint (Collision|BreakHitResult _outhit)) "0, 0,0.000000"))
          (Transformation|SetWorldScale3D _returnvalue_4 (Math|Vector|MakeVector 5.0 5.0 2.5))
          (Variables|/Script/Engine.ParticleSystemComponent|SetCustomTimeDilation _returnvalue_4 0.5)
          (Audio|PlaySoundatLocation "/Game/PrimalEarth/Sound/SFX/HumanMale/WaterSFX/PW_gen_water_splash_heavy_Cue.PW_gen_water_splash_heavy_Cue" (.ImpactPoint (Collision|BreakHitResult _outhit)) 1.0 1.0 0.0 "/Game/PrimalEarth/General/DefaultSoundAttenuationMedium.DefaultSoundAttenuationMedium"))))))

(fn GetCrystalMeshes
  (bind _skullmesh (Variables|Default|GetSkullMesh))
  (Rendering|SetVisibility _skullmesh true false)
  (return (Utilities|Array|MakeArray (Variables|Default|GetCrystalsMesh) _skullmesh (Variables|Default|GetCrystalMesh2) (Variables|Default|GetCrystalMesh3) (Variables|Default|GetCrystalMesh4) (Variables|Default|GetCrystalMesh5) (Variables|Default|GetCrystalMesh1) (Variables|Default|GetStaticMesh6) (Variables|Default|GetStaticMesh5) (Variables|Default|GetStaticMesh4) (Variables|Default|GetStaticMesh3) (Variables|Default|GetStaticMesh1) (Variables|Default|GetStaticMesh2))))